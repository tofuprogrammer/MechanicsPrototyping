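; BP_New_Weapon is a tank weapon that fires arcing projectiles with a short cooldown between shots.
; When triggered while off cooldown, it spawns a half-scale BP_ArcingProjectile at the location and rotation of the tank's DirectionArrow.
; Each shot sets a cooldown flag, which a half-second timer event clears to allow the next shot.
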(event Custom|End%20cooldown
  (Variables|Default|SetWeaponCooldown false))

(event EventTriggered
  (bind _mytank (Variables|Default|GetMyTank))
  (bind _directionarrow (Variables|/Game/Blueprints/BP_PlayerCharacter.BP_PlayerCharacter_C|GetDirectionArrow _mytank))
  (if (not (Variables|Default|GetWeaponCooldown))
    (Game|SpawnActorfromClass "/Game/StudentWork/BP_ArcingProjectile.BP_ArcingProjectile_C" (Math|Transform|MakeTransform (Transformation|GetWorldLocation _directionarrow) (Transformation|GetWorldRotation _directionarrow) "0.500000,0.500000,0.500000") "Undefined" "MultiplyWithRoot" 0 0)
    (Variables|Default|SetWeaponCooldown true)
    (Utilities|Time|SetTimerbyEvent (delegate Custom|End%20cooldown) 0.5)))

(fn ConstructionScript
  (|CallParentFunction))