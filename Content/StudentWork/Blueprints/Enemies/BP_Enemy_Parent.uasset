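; Base enemy Blueprint that targets the player on entering its detection sphere and handles taking damage.
; The overlap stores the player as MyTarget and starts looping timers that call Move and Attack at configurable intervals.
; Move and Attack are empty here, apparently left for child enemies to implement.
; AnyDamage subtracts from health unless EnemyDestroyed is set, destroying the actor at zero or below.
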(event OnComponentBeginOverlap(Sphere)
  (params (OverlappedComponent :type Primitive%20Component%20Object%20Reference) (OtherActor :type Actor%20Object%20Reference) (OtherComp :type Primitive%20Component%20Object%20Reference) (OtherBodyIndex :type Integer) (bFromSweep :type Boolean) (SweepResult :type Hit%20Result%20Structure%20%28by%20ref%29))
  (bind _asbp_player_character (Utilities|Casting|CastToBP_PlayerCharacter OtherActor))
  (Variables|Default|SetMyTarget _asbp_player_character)
  (CallFunction|StartMovementTimer)
  (CallFunction|StartAttackTimer))

(event Custom|Start%20movement%20timer
  (bind _returnvalue (Utilities|Time|SetTimerbyEvent (delegate Custom|Move) (Variables|Default|GetMovementUpdateTime) true))
  (Variables|Default|SetMovement%20Timer _returnvalue))

(event Custom|Move)

(event Custom|Start%20Attack%20Timer
  (bind _returnvalue (Utilities|Time|SetTimerbyEvent (delegate Custom|Attack) (Variables|Default|GetAttack%20Speed) true))
  (Variables|Default|SetAttack%20Timer _returnvalue))

(event Custom|Attack)

(event Game|Damage|EventAnyDamage
  (params (Damage :type Float%20%28single-precision%29) (DamageType :type Damage%20Type%20Object%20Reference) (InstigatedBy :type Controller%20Object%20Reference) (DamageCauser :type Actor%20Object%20Reference))
  (if (not (Variables|Default|GetEnemyDestroyed))
    (Variables|Default|SetCurrentHealth (- (Variables|Default|GetCurrentHealth) Damage))
    (if (<= (Variables|Default|GetCurrentHealth) 0.0)
      (Actor|DestroyActor))))

(fn ConstructionScript)