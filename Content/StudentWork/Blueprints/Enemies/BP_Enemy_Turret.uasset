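; Enemy turret that fires continuously along a fixed arrow component and can be destroyed by damage.
; A looping timer started on BeginPlay spawns turret projectiles at the FireArrow's world location and rotation, with no targeting or range check.
; Incoming damage reduces TurretHealth until the turret plays an explosion sound and Niagara effect, then destroys itself.
; The TurretDestroyed flag gates damage but is never set in these graphs.
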(event Custom|Fire%20projectile
  (bind _firearrow (Variables|Default|GetFireArrow))
  ;[1 0.3 0.3] Attacking
  (Game|SpawnActorfromClass "/Game/StudentWork/Blueprints/Projectiles/BP_Projectile_Enemy_Turret.BP_Projectile_Enemy_Turret_C" (Math|Transform|MakeTransform (Transformation|GetWorldLocation _firearrow) (Transformation|GetWorldRotation _firearrow) "1.000000,1.000000,1.000000") "Undefined" "MultiplyWithRoot" 0 0))

(event Game|Damage|EventAnyDamage
  (params (Damage :type Float%20%28single-precision%29) (DamageType :type Damage%20Type%20Object%20Reference) (InstigatedBy :type Controller%20Object%20Reference) (DamageCauser :type Actor%20Object%20Reference))
  (bind _returnvalue (Transformation|GetActorLocation))
  ;[1 0.3 0.3] Taking damage
  (if (not (Variables|Default|GetTurretDestroyed))
    (Variables|Default|SetTurretHealth (- (Variables|Default|GetTurretHealth) Damage))
    (if (<= (Variables|Default|GetTurretHealth) 0.0)
      (Audio|SpawnSoundatLocation "/Game/StudentWork/Sounds/Explosions/Explosion.Explosion" _returnvalue "0, 0, 0" 1.0 1.0 0.0 0 0)
      (Niagara|SpawnSystematLocation "/Game/StudentWork/Effects/NS_Explosion.NS_Explosion" _returnvalue)
      (Actor|DestroyActor))))

(event EventBeginPlay
  ;[1 0.3 0.3] Attacking
  (bind _returnvalue (Utilities|Time|SetTimerbyEvent (delegate Custom|Fire%20projectile) 0.75 true))
  (Variables|Default|SetFire%20timer _returnvalue))

(fn ConstructionScript)