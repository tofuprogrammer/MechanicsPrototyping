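; BP_Enemy_MoveRandom is an enemy that wanders at random and fires projectiles.
; Its Move event sends the pawn by AI MoveTo to a random reachable navigation point within a radius of its current location.
; Its Attack event spawns a BP_Projectile_Enemy_MoveRandom at the location and rotation of its FireArrow component.
; Neither event is triggered within this Blueprint, and the construction script only calls its parent.
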(event EventAttack
  (bind _firearrow (Variables|Default|GetFireArrow))
  (Game|SpawnActorfromClass "/Game/StudentWork/Blueprints/Projectiles/BP_Projectile_Enemy_MoveRandom.BP_Projectile_Enemy_MoveRandom_C" (Math|Transform|MakeTransform (Transformation|GetWorldLocation _firearrow) (Transformation|GetWorldRotation _firearrow) "1.000000,1.000000,1.000000") "Undefined" "MultiplyWithRoot" 0 0))

(event EventMove
  (AI|AIMoveTo self (.RandomLocation (AI|Navigation|GetRandomReachablePointinRadius (Transformation|GetActorLocation) 1e+03 0 0)) 0 5.0 false))

(fn ConstructionScript
  (|CallParentFunction))