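; BP_Weapon_Rapidfire is a tank weapon that fires small projectiles in quick succession.
; When triggered off cooldown, it spawns a scaled-down BP_Projectile_Rapidfire at the location and rotation of MyTank's DirectionArrow.
; Each shot sets a cooldown flag, which a very short timer clears through EndCooldown to cap the fire rate.
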(event Custom|End%20cooldown
  (Variables|Default|SetWeaponCooldown false))

(event EventTriggered
  (bind _mytank (Variables|Default|GetMyTank))
  (bind _directionarrow (Variables|/Game/Blueprints/BP_PlayerCharacter.BP_PlayerCharacter_C|GetDirectionArrow _mytank))
  (if (not (Variables|Default|GetWeaponCooldown))
    (Game|SpawnActorfromClass "/Game/StudentWork/Blueprints/Projectiles/BP_Projectile_Rapidfire.BP_Projectile_Rapidfire_C" (Math|Transform|MakeTransform (Transformation|GetWorldLocation _directionarrow) (Transformation|GetWorldRotation _directionarrow) "0.500000,0.250000,0.250000") "Undefined" "MultiplyWithRoot" 0 0)
    (Variables|Default|SetWeaponCooldown true)
    (Utilities|Time|SetTimerbyEvent (delegate Custom|End%20cooldown) 0.05)))

(fn ConstructionScript
  (|CallParentFunction))