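; Flamethrower weapon for a player tank that damages whatever is caught in a short sphere sweep ahead of the tank's direction arrow.
; While triggered, it runs a multi-sphere trace and applies damage to each hit, throttled by a brief timer-reset cooldown.
; Starting spawns the Niagara flame attached to the arrow or reactivates the cached one, and completing deactivates it.
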(event Custom|ResetCooldown
  (Variables|Default|SetCooldown? false))

(event EventTriggered
  (bind _mytank (Variables|Default|GetMyTank))
  (bind _directionarrow (Variables|/Game/Blueprints/BP_PlayerCharacter.BP_PlayerCharacter_C|GetDirectionArrow _mytank))
  (bind _returnvalue (Transformation|GetWorldTransform _directionarrow))
  (if (not (Variables|Default|GetCooldown?))
    (bind _outhits (Collision|MultiSphereTraceForObjects (.location _returnvalue) (+ (.location _returnvalue) (* (Math|Vector|GetForwardVector _directionarrow) 2e+02)) 1e+02 (Variables|Default|GetObject%20Types) false 0 "None"))
    (for _array_element _outhits
      (Game|Damage|ApplyDamage (.HitActor (Collision|BreakHitResult _array_element)) 5.0 0 0))
    (Variables|Default|SetCooldown? true)
    (Utilities|Time|SetTimerbyEvent (delegate Custom|ResetCooldown) 0.2)))

(event EventStarted
  (Utilities|IsValid (Variables|Default|GetFlame%20System)
    (:Is%20Valid
      (Components|Activation|Activate (Variables|Default|GetFlame%20System) false))
    (:Is%20Not%20Valid
      (bind _returnvalue (Niagara|SpawnSystemAttached "/Game/StudentWork/Effects/NS_Flamer.NS_Flamer" (Variables|/Game/Blueprints/BP_PlayerCharacter.BP_PlayerCharacter_C|GetDirectionArrow (Variables|Default|GetMyTank)) "None" "0, 0, 0" "0, 0, 0" "KeepRelativeOffset" false))
      (Variables|Default|SetFlame%20System _returnvalue))))

(event EventCompleted
  (Components|Activation|Deactivate (Variables|Default|GetFlame%20System)))

(fn ConstructionScript
  (|CallParentFunction))