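; BP_Target is a destructible target actor that flashes and then explodes when it takes damage.
; The construction script creates a dynamic material instance on its static mesh from a controlled-flash master material.
; The first damage event, gated by DoOnce, plays a timeline that drives the material's FlashLevel parameter.
; When the flash finishes, it plays an explosion sound, spawns an upward mesh-burst Niagara effect and destroys itself.
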(event Game|Damage|EventAnyDamage
  (params (Damage :type Float%20%28single-precision%29) (DamageType :type Damage%20Type%20Object%20Reference) (InstigatedBy :type Controller%20Object%20Reference) (DamageCauser :type Actor%20Object%20Reference))
  (bind _returnvalue (Transformation|GetActorLocation))
  (Utilities|FlowControl|DoOnce false
    (:Completed
      (bind _flash (Timeline|Flash Play)
        (:Update
          (Rendering|Material|SetScalarParameterValue (Variables|Default|GetFlashMaterial) "FlashLevel" _flash :!class /Script/Engine.MaterialInstanceDynamic))
        (:Finished
          (Audio|PlaySoundatLocation "/Game/StudentWork/Sounds/Explosions/Explosion.Explosion" _returnvalue "0, 0, 0" 1.0 1.0 0.0 0 0 0 0)
          (Niagara|SpawnSystematLocation "/Game/StudentWork/Effects/NS_UpwardMeshBurst.NS_UpwardMeshBurst" _returnvalue)
          (Actor|DestroyActor))))))

(fn ConstructionScript
  (bind _returnvalue (Rendering|Material|CreateDynamicMaterialInstance (Variables|Default|GetStaticMesh) 0 "/Game/StudentWork/Materials/MI_ControlledFlash_Master.MI_ControlledFlash_Master" "None" :!class /Script/Engine.PrimitiveComponent))
  (Variables|Default|SetFlashMaterial _returnvalue))